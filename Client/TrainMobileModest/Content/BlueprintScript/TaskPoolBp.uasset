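; TaskPoolBp is a data-access Blueprint that serves task, task script and per-role data from Data Tables.
; Getters return row counts or fetch rows by name or index, most gated on a matching table-name string, covering tasks, role goods, role actions and role first-sight data.
; NotifyRestorFsmFunction separately finds the first top-level GlobeCommunicateWidget and tells its SceneGpjlsz member to restore task scene effects.
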(fn `GetRoleActionsAtRoleName`
  (params (table_name :type String) (role_name :type String))
  (returns (ReturnValue :type "RoleTaskItemAction Structure"))
  (if (`KismetStringLibrary.EqualEqual_StrStr` table_name "RoleTaskItemAction")
    (bind _returnvalue (`|GetDataTableRow` "/Game/TaskData/ScriptContent/OilTankerFire/RoleTaskItemAction.RoleTaskItemAction" (`KismetStringLibrary.Conv_StringToName` role_name))
      (:`then`
        _)
      (:`RowNotFound`
        _)))
  (return _returnvalue))

(fn `GetRoleFirstSightAtRoleName`
  (params (table_name :type String) (role_name :type String))
  (returns (ReturnValue :type "RoleFirstSight Structure"))
  (if (`KismetStringLibrary.EqualEqual_StrStr` table_name "RoleFirstSight")
    (bind _returnvalue (`|GetDataTableRow` "/Game/TaskData/ScriptContent/OilTankerFire/RoleFirstSight.RoleFirstSight" (`KismetStringLibrary.Conv_StringToName` role_name))
      (:`then`
        _)
      (:`RowNotFound`
        _)))
  (return _returnvalue))

(fn `GetRoleGoodsAtRoleName`
  (params (table_name :type String) (role_name :type String))
  (returns (ReturnValue :type "RoleGoodsTexture Structure"))
  (if (`KismetStringLibrary.EqualEqual_StrStr` table_name "RoleTaskItemGoodsTex")
    (bind _returnvalue (`|GetDataTableRow` "/Game/TaskData/ScriptContent/OilTankerFire/RoleTaskItemGoodsTex.RoleTaskItemGoodsTex" (`KismetStringLibrary.Conv_StringToName` role_name))
      (:`then`
        _)
      (:`RowNotFound`
        _)))
  (return _returnvalue))

(fn `GetTaskDataTableAssetAtRow`
  (params (table_name :type String) (row_index :type "Integer (by ref)"))
  (returns (ReturnValue :type "TaskData Structure"))
  (if (`KismetStringLibrary.EqualEqual_StrStr` table_name "TaskData")
    (bind _outrownames (`DataTableFunctionLibrary.GetDataTableRowNames` "/Game/TaskData/ScriptContent/OilTankerFire/TaskData.TaskData"))
    (bind _returnvalue (`|GetDataTableRow` "/Game/TaskData/ScriptContent/OilTankerFire/TaskData.TaskData" (`|GetArrayItem` _outrownames row_index))
      (:`then`
        _)
      (:`RowNotFound`
        _)))
  (return _returnvalue))

(fn `GetTaskDataTableAssetAtRowName`
  (params (table_name :type String) (row_name :type String))
  (returns (ReturnValue :type "TaskData Structure"))
  (if (`KismetStringLibrary.EqualEqual_StrStr` table_name "TaskData")
    (bind _returnvalue (`|GetDataTableRow` "/Game/TaskData/ScriptContent/OilTankerFire/TaskData.TaskData" (`KismetStringLibrary.Conv_StringToName` row_name))
      (:`then`
        _)
      (:`RowNotFound`
        _)))
  (return _returnvalue))

(fn `GetTaskDataTableAssetRowCount`
  (params (table_name :type String))
  (returns (ReturnValue :type Integer))
  (if (`KismetStringLibrary.EqualEqual_StrStr` table_name "TaskData")
    (bind _outrownames (`DataTableFunctionLibrary.GetDataTableRowNames` "/Game/TaskData/ScriptContent/OilTankerFire/TaskData.TaskData")))
  (return (`KismetArrayLibrary.Array_Length` _outrownames)))

(fn `GetTaskScript`
  (params (script_index :type "Integer (by ref)"))
  (returns (ReturnValue :type "ScriptTaskData Structure"))
  (bind _outrownames (`DataTableFunctionLibrary.GetDataTableRowNames` "/Game/TaskData/SriptTaskData.SriptTaskData"))
  (if (> (`KismetArrayLibrary.Array_Length` _outrownames) script_index)
    (bind _returnvalue (`|GetDataTableRow` "/Game/TaskData/SriptTaskData.SriptTaskData" (`|GetArrayItem` _outrownames script_index))
      (:`then`
        _)
      (:`RowNotFound`
        _)))
  (return _returnvalue))

(fn `GetTaskScriptCount`
  (returns (ReturnValue :type Integer))
  (bind _outrownames (`DataTableFunctionLibrary.GetDataTableRowNames` "/Game/TaskData/SriptTaskData.SriptTaskData"))
  (return (`KismetArrayLibrary.Array_Length` _outrownames)))

(fn `NotifyRestorFsmFunction`
  (returns (ReturnValue :type Boolean))
  (`|ExecutionSequence`
    (:`then_0`
      (bind _foundwidgets (`WidgetBlueprintLibrary.GetAllWidgetsOfClass` "/Game/Widget/GlobeCommunicateWidget.GlobeCommunicateWidget_C"))
      (if (> (`KismetArrayLibrary.Array_Length` _foundwidgets) 0)
        (message `/Game/BlueprintScript/ISceneJlsz.NotifyRestoreTaskSceneEffect` (`/Game/Widget/GlobeCommunicateWidget.scene_gpjlsz` (`|GetArrayItem` _foundwidgets)))))
    (:`then_1`
      (return false))))

(fn `UserConstructionScript`)