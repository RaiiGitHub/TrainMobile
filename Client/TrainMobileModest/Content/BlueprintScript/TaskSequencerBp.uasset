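; Task sequencer Blueprint whose functions handle finish, awake and active states of the current task for an FSM, each returning true.
; Each logs a Chinese status message with the current item index from TaskPoolBp to ContentHistoryBp, found through ActorFinder.
; The awake handler also passes the pool's task and item indices to WakeupTaskMessage on the SceneGpjlsz actor.
; Collaborators are looked up by name through FindGlobeActor; the event graph is empty.
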(fn `AddTaskStateMsgToHistory`
  (params (msg :type String))
  (bind _actorfinder (`self.GetActorFinder`))
  (bind _returnvalue (`ActorFinder.FindActor` _actorfinder "ContentHistory"))
  (bind _ascontent_history_bp (cast `/Game/BlueprintScript/ContentHistoryBp` _returnvalue))
  (bind _taskpool (`self.GetTaskPool`))
  (bind _returnvalue_2 (`TaskPool.GetCurrentTaskItemIndex` _taskpool))
  (`DisplayContent.AddContent` _ascontent_history_bp (`KismetStringLibrary.Concat_StrStr` "第" (`KismetStringLibrary.Conv_IntToString` _returnvalue_2) "项任务" msg)))

(fn `GetActorFinder`
  (returns (ActorFinder :type "ActorFinder Object Reference"))
  (bind _returnvalue (`GlobalValueContainer.FindGlobeActor` "ActorFinder"))
  (return (cast `ActorFinder` _returnvalue :!pure true)))

(fn `GetSceneJlsz`
  (returns (scene_actor :type "Actor Object Reference"))
  (bind _returnvalue (`GlobalValueContainer.FindGlobeActor` "SceneGpjlsz"))
  (return _returnvalue))

(fn `GetTaskPool`
  (returns (taskPool :type "TaskPool Object Reference"))
  (bind _returnvalue (`GlobalValueContainer.FindGlobeActor` "TaskPool"))
  (return (cast `/Game/BlueprintScript/TaskPoolBp` _returnvalue :!pure true)))

(fn `SetActiveCurrentTaskFromFsm`
  (returns (ReturnValue :type Boolean))
  (`self.AddTaskStateMsgToHistory` "正在执行。")
  (return true))

(fn `SetAwakeCurrentTaskFromFsm`
  (returns (ReturnValue :type Boolean))
  (`|ExecutionSequence`
    (:`then_0`
      (`self.AddTaskStateMsgToHistory` "已经激活。"))
    (:`then_1`
      (bind _taskpool (`self.GetTaskPool`))
      (bind _returnvalue (`TaskPool.GetCurrentTaskIndex` _taskpool))
      (bind _returnvalue_2 (`TaskPool.GetCurrentTaskItemIndex` _taskpool))
      (`self.WakeUpCommon` _returnvalue _returnvalue_2))
    (:`then_2`
      (return true))))

(fn `SetFinishCurrentTaskFromFsm`
  (returns (ReturnValue :type Boolean))
  (`self.AddTaskStateMsgToHistory` "已被激活，因为前一项任务已经完成。")
  (return true))

(fn `UserConstructionScript`)

(fn `WakeUpCommon`
  (params (taskIndex :type Integer) (itemIndex :type Integer))
  (bind _scene_actor (`self.GetSceneJlsz`))
  (message `/Game/BlueprintScript/ISceneJlsz.WakeupTask` _scene_actor taskIndex itemIndex))