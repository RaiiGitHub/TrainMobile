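; Callback actor for a multiplayer firefighting training drill, routing Notify events to the UI and scene logic.
; It finds widgets by class, using GlobeCommunicateWidget as a hub to forward task, hit and role-switch messages to SceneGpjlsz.
; Other handlers update fire strength, HUD, chat, reconnect and lobby screens, with timers delaying or polling some lobby updates.
; Two events create and find online sessions, logging results through the hub's history logger.
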(event `ReadyToCreateSession`
  (params (sessionIndex :type Integer) (publicConn :type Integer) (useLan :type Boolean))
  (bind _logger (`self.GetLogger`))
  (`DisplayContent.WriteToLog` _logger "entry_func:ready to create session.")
  (bind _returnvalue (`|CreateWidget` "/Game/Widget/SessionWaiting.SessionWaiting_C"))
  (`UserWidget.AddToViewport` _returnvalue 0)
  (`CreateSessionCallbackProxy.CreateSession` (`GameplayStatics.GetPlayerController` 0) publicConn useLan
    (:`then`
      (`Widget.RemoveFromParent` _returnvalue))
    (:`OnSuccess`
      (`DisplayContent.WriteToLog` _logger "create session succeed."))
    (:`OnFailure`
      (`DisplayContent.WriteToLog` _logger "failed to create."))))

(event `RequestToFindSessions`
  (bind _logger (`self.GetLogger`))
  (bind _results (`FindSessionsCallbackProxy.FindSessions` (`GameplayStatics.GetPlayerController` 0) 10 true)
    (:`OnSuccess`
      (`DisplayContent.WriteToLog` _logger "Find Succeed.Result-> \n")
      (for _array_element _results
        (`DisplayContent.WriteToLog` _logger (`KismetStringLibrary.Concat_StrStr` "servername:" (`FindSessionsCallbackProxy.GetServerName` _array_element) " \nping:" (`KismetStringLibrary.Conv_IntToString` (`FindSessionsCallbackProxy.GetPingInMs` _array_element)) " \nmax players:" (`KismetStringLibrary.Conv_IntToString` (`FindSessionsCallbackProxy.GetMaxPlayers` _array_element)) " \ncurrent player:" (`KismetStringLibrary.Conv_IntToString` (`FindSessionsCallbackProxy.GetCurrentPlayers` _array_element))))))
    (:`OnFailure`
      (`DisplayContent.WriteToLog` _logger "Find Session failed."))))

(fn `GetDynamicInstantMatrialTool`
  (returns (dm :type "DynamicInstanceMaterialBuilder Object Reference"))
  (`|ExecutionSequence`
    (:`then_0`
      (bind _foundwidgets (`WidgetBlueprintLibrary.GetAllWidgetsOfClass` "/Game/Widget/GlobeCommunicateWidget.GlobeCommunicateWidget_C"))
      (bind _output (`|GetArrayItem` _foundwidgets))
      (`/Engine/EditorBlueprintResources/StandardMacros.IsValid` _output
        (:`Is Valid`
          (bind _returnvalue (`ActorFinder.FindActor` (cast `ActorFinder` (`/Game/Widget/GlobeCommunicateWidget.ActorFinder` _output) :!pure true) "DynamicInstanceMaterialBuilder"))
          (`/Engine/EditorBlueprintResources/StandardMacros.IsValid` _returnvalue
            (:`Is Valid`
              (return (cast `DynamicInstanceMaterialBuilder` _returnvalue :!pure true)))))))
    (:`then_1`
      (return null))))

(fn `GetLobbyMainHud`
  (returns (lb :type "/Game/Widget/LobbyMainWidget Object Reference"))
  (bind _foundwidgets (`WidgetBlueprintLibrary.GetAllWidgetsOfClass` "/Game/Widget/LobbyMainWidget.LobbyMainWidget_C"))
  (if (> (`KismetArrayLibrary.Array_Length` _foundwidgets) 0)
    (return (`|GetArrayItem` _foundwidgets))
    (else
      (return null))))

(fn `GetLobbyRoleSelectHud`
  (returns (lbr :type "/Game/Widget/LobbyRoleSelectWidget Object Reference"))
  (bind _foundwidgets (`WidgetBlueprintLibrary.GetAllWidgetsOfClass` "/Game/Widget/LobbyRoleSelectWidget.LobbyRoleSelectWidget_C"))
  (if (> (`KismetArrayLibrary.Array_Length` _foundwidgets) 0)
    (return (`|GetArrayItem` _foundwidgets))
    (else
      (return null))))

(fn `GetLogger`
  (returns (logger :type "/Game/BlueprintScript/ContentHistoryBp Object Reference"))
  (bind _foundwidgets (`WidgetBlueprintLibrary.GetAllWidgetsOfClass` "/Game/Widget/GlobeCommunicateWidget.GlobeCommunicateWidget_C"))
  (return (cast `/Game/BlueprintScript/ContentHistoryBp` (`/Game/Widget/GlobeCommunicateWidget.ContentHistory` (`|GetArrayItem` _foundwidgets)) :!pure true)))

(fn `GetMainHud`
  (returns (hud :type "/Game/Widget/MainHudWidget Object Reference"))
  (bind _foundwidgets (`WidgetBlueprintLibrary.GetAllWidgetsOfClass` "/Game/Widget/MainHudWidget.MainHudWidget_C"))
  (if (> (`KismetArrayLibrary.Array_Length` _foundwidgets) 0)
    (return (`|GetArrayItem` _foundwidgets))
    (else
      (return null))))

(fn `GetReconnectHud`
  (returns (ssr :type "/Game/Widget/SocketServerReconnectWidget Object Reference"))
  (bind _foundwidgets (`WidgetBlueprintLibrary.GetAllWidgetsOfClass` "/Game/Widget/SocketServerReconnectWidget.SocketServerReconnectWidget_C"))
  (if (> (`KismetArrayLibrary.Array_Length` _foundwidgets) 0)
    (return (`|GetArrayItem` _foundwidgets))
    (else
      (return null))))

(fn `GetReturnWidget`
  (returns (rw :type "/Game/Widget/ReturnWidget Object Reference"))
  (bind _foundwidgets (`WidgetBlueprintLibrary.GetAllWidgetsOfClass` "/Game/Widget/ReturnWidget.ReturnWidget_C"))
  (return (`|GetArrayItem` _foundwidgets)))

(fn `GetTalkHud`
  (returns (hud :type "/Game/Widget/TalkMsg Object Reference"))
  (bind _foundwidgets (`WidgetBlueprintLibrary.GetAllWidgetsOfClass` "/Game/Widget/TalkMsg.TalkMsg_C"))
  (if (> (`KismetArrayLibrary.Array_Length` _foundwidgets) 0)
    (return (`|GetArrayItem` _foundwidgets))
    (else
      (return null))))

(fn `NotifyActionEffectReplication`
  (params (task_index :type Integer) (item_index :type Integer) (act_index :type Integer) (es :type "EBaseState Enum" :default "BState_INACTIVED"))
  (returns (ReturnValue :type Boolean))
  (`|ExecutionSequence`
    (:`then_0`
      (bind _foundwidgets (`WidgetBlueprintLibrary.GetAllWidgetsOfClass` "/Game/Widget/GlobeCommunicateWidget.GlobeCommunicateWidget_C"))
      (bind _scene_gpjlsz (`/Game/Widget/GlobeCommunicateWidget.scene_gpjlsz` (`|GetArrayItem` _foundwidgets)))
      (`/Engine/EditorBlueprintResources/StandardMacros.IsValid` _scene_gpjlsz
        (:`Is Valid`
          (message `/Game/BlueprintScript/ISceneJlsz.NotifyActionEffectReplication` _scene_gpjlsz task_index item_index act_index es))))
    (:`then_1`
      (return false))))

(fn `NotifyActorMovementDone`
  (params (actor :type "Actor Object Reference"))
  (returns (ReturnValue :type Boolean))
  (`|ExecutionSequence`
    (:`then_0`
      (`/Engine/EditorBlueprintResources/StandardMacros.IsValid` actor
        (:`Is Valid`
          (bind _dm (`self.GetDynamicInstantMatrialTool`))
          (`/Engine/EditorBlueprintResources/StandardMacros.IsValid` _dm
            (:`Is Valid`
              (if (`KismetStringLibrary.EqualEqual_StrStr` (`KismetSystemLibrary.GetObjectName` actor) "AssembleBMWCar")
                (`DynamicInstanceMaterialBuilder.End` _dm "bmw_wheel")))))))
    (:`then_1`
      (return false))))

(fn `NotifyCameraFlyNeedToReset`
  (returns (ReturnValue :type Boolean))
  (`|ExecutionSequence`
    (:`then_0`
      (bind _hud (`self.GetMainHud`))
      (`/Engine/EditorBlueprintResources/StandardMacros.IsValid` _hud
        (:`Is Valid`
          (`/Game/Widget/MainHudWidget.SlidOutDefaultCamera` _hud true))))
    (:`then_1`
      (return false))))

(fn `NotifyCameraFlyToDefaultDone`
  (returns (ReturnValue :type Boolean))
  (`|ExecutionSequence`
    (:`then_0`
      (bind _hud (`self.GetMainHud`))
      (`/Game/Widget/MainHudWidget.SlidOutDefaultCamera` _hud false))
    (:`then_1`
      (return false))))

(fn `NotifyFirePercent`
  (params (percent :type "Float (double-precision)") (ReachTargetPercent :type Integer))
  (returns (ReturnValue :type Boolean))
  (locals (CurDesc :type String))
  (bind _foundwidgets (`WidgetBlueprintLibrary.GetAllWidgetsOfClass` "/Game/Widget/FireStrengthWidget.FireStrengthWidget_C"))
  (bind _output (`|GetArrayItem` _foundwidgets))
  (set `/Game/Widget/FireStrengthWidget.fire_percent` percent _output)
  (switch `int` ReachTargetPercent
    (:`Default`
      _)
    (:`0`
      (set `local.CurDesc` "正在灭火"))
    (:`1`
      (set `local.CurDesc` "需要协助")
      (`/Game/Widget/FireStrengthWidget.FlickerNotification` _output 3)
      (add `/Game/Widget/FireStrengthWidget.FlickerAniComplete` _output (`|CreateDelegate` :!event `NotifyFirePercentFlickerDone`)))
    (:`2`
      (set `local.CurDesc` "火势变大")))
  (set `/Game/Widget/FireStrengthWidget.info_desc` (`local.CurDesc`) _output)
  (return true))

(fn `NotifyFirePercentFlickerDone`
  (bind _foundwidgets (`WidgetBlueprintLibrary.GetAllWidgetsOfClass` "/Game/Widget/GlobeCommunicateWidget.GlobeCommunicateWidget_C"))
  (bind _output (`|GetArrayItem` _foundwidgets))
  (bind _returnvalue (`PawnHandler.GetCurrentHandlePawn` (cast `PawnHandler` (`/Game/Widget/GlobeCommunicateWidget.PawnHandler` _output) :!pure true)))
  (if (== _returnvalue (`GameplayStatics.GetPlayerPawn` 0))
    (bind _returnvalue_2 (`TaskPool.GetCurrentRoleIndex` (cast `TaskPool` (`/Game/Widget/GlobeCommunicateWidget.TaskPool` _output) :!pure true)))
    (switch `int` _returnvalue_2
      (:`2`
        (bind _scene_gpjlsz (`/Game/Widget/GlobeCommunicateWidget.scene_gpjlsz` _output))
        (message `/Game/BlueprintScript/ISceneJlsz.NotifyRoleSwitch` _scene_gpjlsz 1 2 5))
      (:`3`
        (message `/Game/BlueprintScript/ISceneJlsz.NotifyRoleSwitch` _scene_gpjlsz 1 3 5))
      (:`5`
        (message `/Game/BlueprintScript/ISceneJlsz.NotifyRoleSwitch` _scene_gpjlsz 1 5 4)))))

(fn `NotifyHappyEnding`
  (returns (ReturnValue :type Boolean))
  (`|ExecutionSequence`
    (:`then_0`
      (bind _hud (`self.GetMainHud`))
      (`/Game/Widget/MainHudWidget.HappyEnding` _hud))
    (:`then_1`
      (return false))))

(fn `NotifyHitResult`
  (returns (ReturnValue :type Boolean))
  (bind _foundwidgets (`WidgetBlueprintLibrary.GetAllWidgetsOfClass` "/Game/Widget/GlobeCommunicateWidget.GlobeCommunicateWidget_C"))
  (bind _succeed (message `/Game/BlueprintScript/ISceneJlsz.NotifyHitEvent` (`/Game/Widget/GlobeCommunicateWidget.scene_gpjlsz` (`|GetArrayItem` _foundwidgets))))
  (return _succeed))

(fn `NotifyHitResultFree`
  (params (hr :type "HitResult Structure (by ref)"))
  (returns (ReturnValue :type Boolean))
  (bind _foundwidgets (`WidgetBlueprintLibrary.GetAllWidgetsOfClass` "/Game/Widget/GlobeCommunicateWidget.GlobeCommunicateWidget_C"))
  (bind _succeed (message `/Game/BlueprintScript/ISceneJlsz.NotifyHitResult` (`/Game/Widget/GlobeCommunicateWidget.scene_gpjlsz` (`|GetArrayItem` _foundwidgets)) hr))
  (return _succeed))

(fn `NotifyLobbyLaunchedOn`
  (returns (ReturnValue :type Boolean))
  (`|ExecutionSequence`
    (:`then_0`
      (`self.PrepareToLaunchOnGameTimer`))
    (:`then_1`
      (return false))))

(fn `NotifyLobbyReadyAsked`
  (returns (ReturnValue :type Boolean))
  (`|ExecutionSequence`
    (:`then_0`
      (`KismetSystemLibrary.K2_SetTimer` null "PopReadyAskPanelTimer" 1.0))
    (:`then_1`
      (return false))))

(fn `NotifyLobbyRoleSelectFinished`
  (params (finished :type Boolean))
  (returns (ReturnValue :type Boolean))
  (`|ExecutionSequence`
    (:`then_0`
      (bind _foundwidgets (`WidgetBlueprintLibrary.GetAllWidgetsOfClass` "/Game/Widget/LobbyRoleSelectWidget.LobbyRoleSelectWidget_C"))
      (if finished
        (`Widget.RemoveFromParent` _foundwidgets)
        (bind _foundwidgets_2 (`WidgetBlueprintLibrary.GetAllWidgetsOfClass` "/Game/Widget/ReturnWidget.ReturnWidget_C"))
        (bind _output (`|GetArrayItem` _foundwidgets_2))
        (set `/Game/Widget/ReturnWidget.WidgetLevel` 5 _output)
        (`/Game/Widget/ReturnWidget.DoAllTaskAgain` _output)
        (elif (> (`KismetArrayLibrary.Array_Length` _foundwidgets) 0)
          (`/Game/Widget/LobbyRoleSelectWidget.UpdateRoleSelectFinishBrush` (`|GetArrayItem` _foundwidgets)))))
    (:`then_1`
      (return false))))

(fn `NotifyLobbyUpdate`
  (returns (ReturnValue :type Boolean))
  (`|ExecutionSequence`
    (:`then_0`
      (bind _lb (`self.GetLobbyMainHud`))
      (`/Engine/EditorBlueprintResources/StandardMacros.IsValid` _lb
        (:`Is Valid`
          (`KismetSystemLibrary.K2_SetTimer` null "UpdateLobbyPanelTimer" 1.0 true))
        (:`Is Not Valid`
          (bind _lbr (`self.GetLobbyRoleSelectHud`))
          (`/Engine/EditorBlueprintResources/StandardMacros.IsValid` _lbr
            (:`Is Valid`
              (`/Game/Widget/LobbyRoleSelectWidget.UpdateRoleSlot` _lbr)
              (`/Game/Widget/LobbyRoleSelectWidget.CheckBtnStartEnable` _lbr))))))
    (:`then_1`
      (return false))))

(fn `NotifyMatchLobbyTryMaxTime`
  (returns (ReturnValue :type Boolean))
  (`|ExecutionSequence`
    (:`then_0`
      (bind _lb (`self.GetLobbyMainHud`))
      (`/Engine/EditorBlueprintResources/StandardMacros.IsValid` _lb
        (:`Is Valid`
          (`/Game/Widget/LobbyMainWidget.ShowMsgBox` _lb true "没有队伍" "现在没有创建好的队伍。" true false 0 "" "")
          (`/Game/Widget/LobbyMainWidget.btn_create_lobby_click` _lb))))
    (:`then_1`
      (return false))))

(fn `NotifyMessageRecieve`
  (params (msg :type String) (from_uid :type String) (from_uname :type String) (em :type "ETalkMessageType Enum" :default "E_MSG_WORLD"))
  (returns (ReturnValue :type Boolean))
  (locals (tw :type "/Game/Widget/TalkMsg Object Reference") (tex_path :type String :default "Texture2D'/Game/UITEXTURE/QianStyle/qian_default.qian_default'"))
  (`|ExecutionSequence`
    (:`then_0`
      (bind (_role_name _returnvalue) (`TrainGameInstance.GetRoleNameAsUserID` (cast `TrainGameInstance` (`GameplayStatics.GetGameInstance`) :!pure true) ""))
      (if _returnvalue
        (bind _returnvalue_2 (`|GetDataTableRow` "/Game/TaskData/ScriptContent/OilTankerFire/PicAniData.PicAniData" (`KismetStringLibrary.Conv_StringToName` _role_name))
          (:`then`
            (set `local.tex_path` (`.HeadPortraitPath` (break `RoleImageData` _returnvalue_2)))))))
    (:`then_1`
      (bind _lbr (`self.GetLobbyRoleSelectHud`))
      (`/Engine/EditorBlueprintResources/StandardMacros.IsValid` _lbr
        (:`Is Valid`
          (`/Game/Widget/LobbyRoleSelectWidget.AddMessage` _lbr msg from_uname)
          (return false))))
    (:`then_2`
      (`|ExecutionSequence`
        (:`then_0`
          (bind _hud (`self.GetTalkHud`))
          (bind _output_get (set `local.tw` _hud))
          (`/Engine/EditorBlueprintResources/StandardMacros.IsValid` _output_get
            (:`Is Not Valid`
              (bind _returnvalue_3 (`|CreateWidget` "/Game/Widget/TalkMsg.TalkMsg_C"))
              (`UserWidget.AddToViewport` _returnvalue_3 0)
              (`Widget.SetVisibility` _returnvalue_3 "Hidden")
              (set `local.tw` _returnvalue_3))))
        (:`then_1`
          (switch `ETalkMessageType` em
            (:`E_MSG_WORLD`
              (`/Game/Widget/TalkMsg.AddMessage` (`local.tw`) false msg false from_uname (`local.tex_path`)))
            (:`E_MSG_TEAM`
              (`/Game/Widget/TalkMsg.AddMessage` (`local.tw`) false msg true from_uname (`local.tex_path`)))))))
    (:`then_3`
      (return false))))

(fn `NotifyReachedTarget`
  (params (task_index :type Integer) (item_index :type Integer) (act_index :type Integer) (aspect_name :type String) (mesh_name :type String))
  (returns (ReturnValue :type Boolean))
  (bind _foundwidgets (`WidgetBlueprintLibrary.GetAllWidgetsOfClass` "/Game/Widget/GlobeCommunicateWidget.GlobeCommunicateWidget_C"))
  (bind _bsucceed (message `/Game/BlueprintScript/ISceneJlsz.NotifyReachActionPos` (`/Game/Widget/GlobeCommunicateWidget.scene_gpjlsz` (`|GetArrayItem` _foundwidgets)) task_index item_index act_index aspect_name mesh_name))
  (return _bsucceed))

(fn `NotifyScrollMessage`
  (params (msg :type String) (positive :type Boolean) (scroll_rate :type "Float (double-precision)"))
  (returns (ReturnValue :type Boolean))
  (`|ExecutionSequence`
    (:`then_0`
      (bind _hud (`self.GetMainHud`))
      (`/Engine/EditorBlueprintResources/StandardMacros.IsValid` _hud
        (:`Is Valid`
          (`/Game/Widget/MainHudWidget.PopScrollBillboard` _hud msg positive scroll_rate))))
    (:`then_1`
      (return false))))

(fn `NotifySocketServerReconnect`
  (params (essr :type "ESocketServerReconnect Enum" :default "E_RECONNECT_NO_NEED"))
  (returns (ReturnValue :type Boolean))
  (`|ExecutionSequence`
    (:`then_0`
      (switch `ESocketServerReconnect` essr
        (:`E_RECONNECT_TRY`
          (bind _ssr (`self.GetReconnectHud`))
          (`/Engine/EditorBlueprintResources/StandardMacros.IsValid` _ssr
            (:`Is Not Valid`
              (bind _returnvalue (`|CreateWidget` "/Game/Widget/SocketServerReconnectWidget.SocketServerReconnectWidget_C"))
              (`UserWidget.AddToViewport` _returnvalue 520))))
        (:`E_RECONNECT_OK`
          (bind _ssr_2 (`self.GetReconnectHud`))
          (`/Engine/EditorBlueprintResources/StandardMacros.IsValid` _ssr_2
            (:`Is Valid`
              (`/Game/Widget/SocketServerReconnectWidget.Reconnected` _ssr_2))))))
    (:`then_1`
      (return false))))

(fn `NotifyTaskCanPassbyRecieve`
  (params (task_index :type Integer) (item_index :type Integer) (act_index :type Integer) (pending_es :type "EBaseState Enum" :default "BState_INACTIVED"))
  (returns (ReturnValue :type Boolean))
  (`|ExecutionSequence`
    (:`then_0`
      (bind _foundwidgets (`WidgetBlueprintLibrary.GetAllWidgetsOfClass` "/Game/Widget/GlobeCommunicateWidget.GlobeCommunicateWidget_C"))
      (bind _scene_gpjlsz (`/Game/Widget/GlobeCommunicateWidget.scene_gpjlsz` (`|GetArrayItem` _foundwidgets)))
      (`/Engine/EditorBlueprintResources/StandardMacros.IsValid` _scene_gpjlsz
        (:`Is Valid`
          (message `/Game/BlueprintScript/ISceneJlsz.NotifyTaskCanPassbyRecieve` _scene_gpjlsz task_index item_index act_index pending_es))))
    (:`then_1`
      (return false))))

(fn `NotifyTaskItemActionStateChanged`
  (params (task_index :type Integer) (item_index :type Integer) (act_index :type Integer) (es :type "EBaseState Enum" :default "BState_INACTIVED") (op_desc :type String))
  (returns (ReturnValue :type Boolean))
  (`|ExecutionSequence`
    (:`then_0`
      (bind _foundwidgets (`WidgetBlueprintLibrary.GetAllWidgetsOfClass` "/Game/Widget/GlobeCommunicateWidget.GlobeCommunicateWidget_C")))
    (:`then_1`
      (switch `EBaseState` es
        (:`BState_ACTIVED`
          (bind _scene_gpjlsz (`/Game/Widget/GlobeCommunicateWidget.scene_gpjlsz` (`|GetArrayItem` _foundwidgets)))
          (message `/Game/BlueprintScript/ISceneJlsz.NotifyActiveTaskItemAction` _scene_gpjlsz task_index item_index act_index))
        (:`BState_FINISHED`
          (message `/Game/BlueprintScript/ISceneJlsz.NotifyMissionDone` _scene_gpjlsz task_index item_index act_index))))
    (:`then_2`
      (bind _hud (`self.GetMainHud`))
      (bind _ai (`/Game/Widget/MainHudWidget.GetActionIllustration` _hud))
      (`/Engine/EditorBlueprintResources/StandardMacros.IsValid` _ai
        (:`Is Valid`
          (`/Game/Widget/ActionIllustration.Update` _ai))))
    (:`then_3`
      (return false))))

(fn `PopReadyAskPanelTimer`
  (bind _lb (`self.GetLobbyMainHud`))
  (`/Game/Widget/LobbyMainWidget.ReadyAni` _lb true)
  (`/Game/Widget/LobbyMainWidget.ShowMsgBox` _lb true "队伍就绪" "演练已就绪，您准备好了吗？" true true 2 "" "")
  (`KismetSystemLibrary.K2_ClearTimer` null "PopReadyAskPanelTimer"))

(fn `PrepareToLaunchOnGameTimer`
  (bind _lb (`self.GetLobbyMainHud`))
  (`Widget.RemoveFromParent` _lb)
  (bind _returnvalue (`|CreateWidget` "/Game/Widget/LobbyRoleSelectWidget.LobbyRoleSelectWidget_C"))
  (`UserWidget.AddToViewport` _returnvalue 0))

(fn `UpdateLobbyPanelTimer`
  (bind _lb (`self.GetLobbyMainHud`))
  (`/Engine/EditorBlueprintResources/StandardMacros.IsValid` _lb
    (:`Is Valid`
      (bind _ok (`/Game/Widget/LobbyMainWidget.UpdateMemberSlot` _lb))
      (if _ok
        (`KismetSystemLibrary.K2_ClearTimer` null "UpdateLobbyPanelTimer")))))

(fn `UserConstructionScript`)