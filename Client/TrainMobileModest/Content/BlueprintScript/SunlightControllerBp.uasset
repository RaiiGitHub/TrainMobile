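; Sunlight controller that exposes setters for the level's BP_Sky_Sphere: zenith, overall and cloud colors, horizon falloff and sun height.
; Each call looks up the sky sphere by name through the ActorFinder on the first top-level GlobeCommunicateWidget.
; Setters apply their value, then call UpdateSunDirection to refresh the sky.
; Sun height maps a normalized value to the directional light's pitch over a full, inverted turn.
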(fn `GetSkySphere`
  (returns (SkySphere :type "/Engine/EngineSky/BP_Sky_Sphere Object Reference"))
  (bind _foundwidgets (`WidgetBlueprintLibrary.GetAllWidgetsOfClass` "/Game/Widget/GlobeCommunicateWidget.GlobeCommunicateWidget_C"))
  (bind _item (`KismetArrayLibrary.Array_Get` _foundwidgets))
  (`/Engine/EditorBlueprintResources/StandardMacros.IsValid` _item
    (:`Is Valid`
      (bind _returnvalue (`ActorFinder.FindActor` (cast `ActorFinder` (`/Game/Widget/GlobeCommunicateWidget.ActorFinder` _item) :!pure true) "BP_Sky_Sphere"))
      (bind _asbp_sky_sphere (cast `/Engine/EngineSky/BP_Sky_Sphere` _returnvalue)
        (:`then`
          _)
        (:`CastFailed`
          _))
      (return _asbp_sky_sphere))))

(fn `SetCloudColor`
  (params (color :type "LinearColor Structure"))
  (returns (ReturnValue :type Boolean))
  (bind _skysphere (`self.GetSkySphere`))
  (`/Engine/EditorBlueprintResources/StandardMacros.IsValid` _skysphere
    (:`Is Valid`
      (set `/Engine/EngineSky/BP_Sky_Sphere.Cloud color` color _skysphere)
      (`/Engine/EngineSky/BP_Sky_Sphere.UpdateSunDirection` _skysphere))
    (:`Is Not Valid`
      _))
  (return true))

(fn `SetHorizonFallOff`
  (params (horizonFalloff :type "Float (double-precision)"))
  (returns (ReturnValue :type Boolean))
  (bind _skysphere (`self.GetSkySphere`))
  (`/Engine/EditorBlueprintResources/StandardMacros.IsValid` _skysphere
    (:`Is Valid`
      (set `/Engine/EngineSky/BP_Sky_Sphere.Horizon Falloff` horizonFalloff _skysphere)
      (`/Engine/EngineSky/BP_Sky_Sphere.UpdateSunDirection` _skysphere))
    (:`Is Not Valid`
      _))
  (return true))

(fn `SetOverallColor`
  (params (color :type "LinearColor Structure"))
  (returns (ReturnValue :type Boolean))
  (bind _skysphere (`self.GetSkySphere`))
  (`/Engine/EditorBlueprintResources/StandardMacros.IsValid` _skysphere
    (:`Is Valid`
      (set `/Engine/EngineSky/BP_Sky_Sphere.Overall Color` color _skysphere)
      (`/Engine/EngineSky/BP_Sky_Sphere.UpdateSunDirection` _skysphere))
    (:`Is Not Valid`
      _))
  (return true))

(fn `SetSunHeight`
  (params (sunHeight :type "Float (double-precision)"))
  (returns (ReturnValue :type Boolean))
  (bind _skysphere (`self.GetSkySphere`))
  (`/Engine/EditorBlueprintResources/StandardMacros.IsValid` _skysphere
    (:`Is Valid`
      (`self.K2_SetActorRotation` (`/Engine/EngineSky/BP_Sky_Sphere.Directional light actor` _skysphere) (`KismetMathLibrary.MakeRotator` 0.0 (`KismetMathLibrary.MapRangeUnclamped` sunHeight 0.0 1.0 360.0 0.0) 0.0) false)
      (`/Engine/EngineSky/BP_Sky_Sphere.UpdateSunDirection` _skysphere))
    (:`Is Not Valid`
      _))
  (return true))

(fn `SetZenithColor`
  (params (color :type "LinearColor Structure"))
  (returns (ReturnValue :type Boolean))
  (bind _skysphere (`self.GetSkySphere`))
  (`/Engine/EditorBlueprintResources/StandardMacros.IsValid` _skysphere
    (:`Is Valid`
      (set `/Engine/EngineSky/BP_Sky_Sphere.Zenith Color` color _skysphere)
      (`/Engine/EngineSky/BP_Sky_Sphere.UpdateSunDirection` _skysphere))
    (:`Is Not Valid`
      _))
  (return true))

(fn `UserConstructionScript`)