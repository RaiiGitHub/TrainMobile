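; Online notification handler for the Train game that turns socket and HTTP server results into UI responses and follow-up requests.
; On socket connect it sends a handshake through TrainGameInstance, setting up the receiver only on first connection.
; Notify callbacks find register, login and HUD widgets by class to show results, advance screens or open a download overlay after version verification.
; Ready team results are uploaded, then the happy ending plays and is dispatched to lobby members.
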(event `self.NotifySocketServerConnected`
  (params (user_id :type String) (socket_name :type String) (recon :type Boolean))
  (bind _astrain_game_instance (cast `TrainGameInstance` (`GameplayStatics.GetGameInstance`) :!pure true))
  (if (not recon)
    (`TrainGameInstance.SetupSocketReciever` _astrain_game_instance socket_name))
  (bind _returnvalue (`TrainGameInstance.BuildHandshakeString` _astrain_game_instance))
  (`TrainGameInstance.SendDataToSocketServer` _astrain_game_instance socket_name _returnvalue "handshake" true))

(event `self.NotifyUserRankDataReady`
  (bind _astrain_game_instance (cast `TrainGameInstance` (`GameplayStatics.GetGameInstance`) :!pure true))
  (bind _returnvalue (`TrainGameInstance.GetCurrentLobbyResult` _astrain_game_instance))
  (`TrainGameInstance.VisitUrlWithGetMethod` _astrain_game_instance (`KismetStringLibrary.Concat_StrStr` "fs_user_upload_team.php?data=" _returnvalue) "user_upload_team") ; upload this team data to the server.
)

(event `self.NotifyUserRankDataUploaded`
  (bind _hud (`self.GetMainHud`))
  (`/Game/Widget/MainHudWidget.HappyEnding` _hud)
  (`TrainGameInstance.DispatchMsgToLobbyMember` (cast `TrainGameInstance` (`GameplayStatics.GetGameInstance`) :!pure true) "taskcomplete-happy-ending-please" false))

(fn `GetMainHud`
  (returns (hud :type "/Game/Widget/MainHudWidget Object Reference"))
  (bind _foundwidgets (`WidgetBlueprintLibrary.GetAllWidgetsOfClass` "/Game/Widget/MainHudWidget.MainHudWidget_C"))
  (if (> (`KismetArrayLibrary.Array_Length` _foundwidgets) 0)
    (return (`KismetArrayLibrary.Array_Get` _foundwidgets))
    (else
      (return null))))

(fn `NotifyHandshake`
  (params (msg :type String) (shake :type Boolean))
  (returns (ReturnValue :type Boolean))
  (`|ExecutionSequence`
    (:`then_0`
      (if (`KismetStringLibrary.Contains` msg "handshake")
        (bind _foundwidgets (`WidgetBlueprintLibrary.GetAllWidgetsOfClass` "/Game/Widget/UserLogin.UserLogin_C"))
        (if shake
          (`/Game/Widget/UserLogin.EnterRegister` (`KismetArrayLibrary.Array_Get` _foundwidgets)))))
    (:`then_1`
      (return false))))

(fn `NotifyHttpRequestErr`
  (params (msg :type String))
  (returns (ReturnValue :type Boolean))
  (`|ExecutionSequence`
    (:`then_0`
      (if (or (`KismetStringLibrary.Contains` msg "login") (`KismetStringLibrary.Contains` msg "handshake"))
        (bind _foundwidgets (`WidgetBlueprintLibrary.GetAllWidgetsOfClass` "/Game/Widget/UserLogin.UserLogin_C"))
        (`/Game/Widget/UserLogin.ShowMsgSimple` (`KismetArrayLibrary.Array_Get` _foundwidgets) "没有连接" "检查您的网络和服务器设置。" null)))
    (:`then_1`
      (return false))))

(fn `NotifyLoginMsg`
  (params (ls :type "ELoginStatus Enum" :default "LS_PERMISSION_FAILED"))
  (returns (ReturnValue :type Boolean))
  (bind _foundwidgets (`WidgetBlueprintLibrary.GetAllWidgetsOfClass` "/Game/Widget/UserLogin.UserLogin_C"))
  (`|ExecutionSequence`
    (:`then_0`
      (switch `ELoginStatus` ls
        (:`LS_PERMISSION_FAILED`
          (bind _item (`KismetArrayLibrary.Array_Get` _foundwidgets))
          (`/Game/Widget/UserLogin.ShowMsgSimple` _item "提示" "账号或者密码不正确" null)
          (`/Game/Widget/UserLogin.ShowLogining` _item false))
        (:`LS_PERMISSION_TOTAL`
          (`/Game/Widget/UserLogin.SaveUserLoginInfo` _item true)
          (bind _returnvalue (`TrainGameInstance.VersionVerify` (cast `TrainGameInstance` (`GameplayStatics.GetGameInstance`) :!pure true)))
          (if _returnvalue
            (bind _returnvalue_2 (`|CreateWidget` "/Game/Widget/LoadingWidget.LoadingWidget_C"))
            (`UserWidget.AddToViewport` _returnvalue_2 0)
            (set `/Game/Widget/LoadingWidget.vis` "Visible" _returnvalue_2)
            (set `/Game/Widget/LoadingWidget.info` "下载中(0.0%)" _returnvalue_2)
            (else
              (`/Game/Widget/UserLogin.EnterMainMenu` _item))))))
    (:`then_1`
      (return false))))

(fn `NotifyRegisterMsg`
  (params (success :type Boolean))
  (returns (ReturnValue :type Boolean))
  (`|ExecutionSequence`
    (:`then_0`
      (bind _foundwidgets (`WidgetBlueprintLibrary.GetAllWidgetsOfClass` "/Game/Widget/UserRegister.UserRegister_C")))
    (:`then_1`
      (if success
        (bind _item (`KismetArrayLibrary.Array_Get` _foundwidgets))
        (`/Game/Widget/UserRegister.ShowMsgSimple` _item "欢迎" "已成功注册，立即去登陆吧。" _item)
        (else
          (`/Game/Widget/UserRegister.ShowMsgSimple` _item "糟糕" "现在还不能注册。" null))))
    (:`then_2`
      (return false))))

(fn `NotifyUpdateUserExp`
  (returns (ReturnValue :type Boolean))
  (bind _foundwidgets (`WidgetBlueprintLibrary.GetAllWidgetsOfClass` "/Game/Widget/MainHudWidget.MainHudWidget_C"))
  (`/Game/Widget/MainHudWidget.UpdateUserInfo` (`KismetArrayLibrary.Array_Get` _foundwidgets))
  (return false))

(fn `NotifyUserIDExistVerify`
  (params (id :type String) (exist :type Boolean))
  (returns (ReturnValue :type Boolean))
  (`|ExecutionSequence`
    (:`then_0`
      (bind _foundwidgets (`WidgetBlueprintLibrary.GetAllWidgetsOfClass` "/Game/Widget/UserRegister.UserRegister_C"))
      (if exist
        (bind _item (`KismetArrayLibrary.Array_Get` _foundwidgets))
        (`/Game/Widget/UserRegister.ShowMsgSimple` _item "用户已存在" (`KismetStringLibrary.Concat_StrStr` "\"" id "\"" "已经被注册了。") null)
        (else
          (`/Game/Widget/UserRegister.PutKeyValInClientUser` _item 1)
          (`/Game/Widget/UserRegister.EmptyTextBox` _item)
          (`/Game/Widget/UserRegister.SetupDisplayInfo` _item 2)
          (`/Game/Widget/UserRegister.SetStep` _item 2)
          (`/Game/Widget/UserRegister.SetupTextboxValue` _item 2))))
    (:`then_1`
      (return false))))

(fn `UserConstructionScript`)